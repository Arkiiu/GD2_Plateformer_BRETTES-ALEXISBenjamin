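; BPC_Collect is a Blueprint component that applies collectible pickups to the player's score and bonus charge stored in BP_GameInstance.
; It caches the game instance on BeginPlay.
; Collect adds the item's value, scaled by the score multiplier, then destroys the item.
; CollectBonus adds bonus charge, destroying the item only if the total stays below six; otherwise it sets the charge to five and leaves the item intact.
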(event `self.ReceiveBeginPlay`
  (bind _asbp_game_instance (cast `/Game/Blueprint/BP_GameInstance` (`GameplayStatics.GetGameInstance`)))
  (set `self.BP Game Instance` _asbp_game_instance))

(fn `Collect`
  (params (Collectible :type "/Game/Blueprint/BPC_Collectible Object Reference"))
  (bind _bp_game_instance (`self.BP Game Instance`))
  (set `/Game/Blueprint/BP_GameInstance.PlayerScore` (+ (* (`/Game/Blueprint/BPC_Collectible.Value` Collectible) (`/Game/Blueprint/BP_GameInstance.PlayerScoreMultiplier` _bp_game_instance)) (`/Game/Blueprint/BP_GameInstance.PlayerScore` _bp_game_instance)) _bp_game_instance)
  (`/Game/Blueprint/BPC_Collectible.DestroyBPCollectible` Collectible))

(fn `CollectBonus`
  (params (Collectible :type "/Game/Blueprint/BPC_CollectibleBonus Object Reference"))
  (bind _bp_game_instance (`self.BP Game Instance`))
  (bind _output_get (set `/Game/Blueprint/BP_GameInstance.BonusCharge` (+ (`/Game/Blueprint/BPC_CollectibleBonus.BonusValue` Collectible) (`/Game/Blueprint/BP_GameInstance.BonusCharge` _bp_game_instance)) _bp_game_instance))
  (if (not (>= _output_get 6))
    (`/Game/Blueprint/BPC_CollectibleBonus.DestroyBPCollectible` Collectible)
    (else
      (set `/Game/Blueprint/BP_GameInstance.BonusCharge` 5 _bp_game_instance))))