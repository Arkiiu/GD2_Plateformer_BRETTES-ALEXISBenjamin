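; Button actor that toggles the platform activation state shared through the game instance.
; On BeginPlay it caches BP_GameInstance and binds its ButtonPressed event through the instance's BindEventToButtonPress.
; Each press alternates via a FlipFlop, setting Cube2's material to green and ActivatePlateform to true, or to blue and false.
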(event `self.ReceiveBeginPlay`
  (bind _asbp_game_instance (cast `/Game/Blueprint/BP_GameInstance` (`GameplayStatics.GetGameInstance`)))
  (set `self.BP Game Instance` _asbp_game_instance)
  (add `/Game/Blueprint/BP_GameInstance.ButtonPress` (`self.BP Game Instance`) (delegate `ButtonPressed`)))

(event `ButtonPressed`
  (bind _bp_game_instance (`self.BP Game Instance`))
  (bind _cube2 (`self.Cube2`))
  (`/Engine/EditorBlueprintResources/StandardMacros.FlipFlop`
    (:`A`
      (`PrimitiveComponent.SetMaterial` _cube2 0 "/Game/LevelPrototyping/Materials/MI_Solid_Green.MI_Solid_Green")
      (set `/Game/Blueprint/BP_GameInstance.ActivatePlateform` true _bp_game_instance))
    (:`B`
      (`PrimitiveComponent.SetMaterial` _cube2 0 "/Game/LevelPrototyping/Materials/MI_Solid_Blue.MI_Solid_Blue")
      (set `/Game/Blueprint/BP_GameInstance.ActivatePlateform` false _bp_game_instance))))

(fn `UserConstructionScript`)