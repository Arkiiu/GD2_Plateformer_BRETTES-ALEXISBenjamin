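; BP_MovingPlateform2 is a moving platform for the Level 3 parkour.
; On BeginPlay it caches the game instance and its start location, then plays the Move timeline only if ActivateLevel3Parkour is set.
; The timeline linearly blends the root vertically from its start toward a fixed world height, keeping X and Y and teleporting without sweep.
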(event `self.ReceiveBeginPlay`
  (bind _defaultsceneroot (`self.DefaultSceneRoot`))
  (bind _startloc (`self.StartLoc`))
  (bind _asbp_game_instance (cast `/Game/Blueprint/BP_GameInstance` (`GameplayStatics.GetGameInstance`)))
  (set `self.BP Game Instance` _asbp_game_instance)
  (set `self.StartLoc` (`SceneComponent.K2_GetComponentLocation` _defaultsceneroot))
  (if (`/Game/Blueprint/BP_GameInstance.ActivateLevel3Parkour` (`self.BP Game Instance`))
    (bind (_direction _newtrack_0) (`Timeline|Move` :!via `PlayFromStart`)
      (:`Update`
        (`SceneComponent.K2_SetWorldLocation` _defaultsceneroot (`|EaseFunction` "Linear" _newtrack_0 _startloc (`KismetMathLibrary.MakeVector` (.x _startloc) (.y _startloc) 40.0)) false true)))))

(fn `UserConstructionScript`)